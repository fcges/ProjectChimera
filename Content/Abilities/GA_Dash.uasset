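; Gameplay ability that makes BP_CombatCharacter dash by temporarily overriding its movement and hiding its mesh.
; It passes dash distance and rate to the character, caches movement settings, then sets max speed to their product with near-instant acceleration and turning.
; After a short delay compensated for time-stop dilation, it sends DashTag to the character.
; On the EndDash event, the shared DashSetup function restores movement and visibility, and the ability ends.
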(event `self.K2_ActivateAbility`
  (bind _dash_distance (`self.Dash_Distance`))
  (bind _dash_rate (`self.Dash_Rate`))
  (bind _asbp_combat_character (cast `/Game/Variant_Combat/Blueprints/BP_CombatCharacter` (`self.GetAvatarActorFromActorInfo`)))
  (set `/Game/Variant_Combat/Blueprints/BP_CombatCharacter.Dash_Distance` _dash_distance _asbp_combat_character)
  (set `/Game/Variant_Combat/Blueprints/BP_CombatCharacter.Dash_Rate` _dash_rate _asbp_combat_character)
  (bind _charactermovement (`Character.CharacterMovement` _asbp_combat_character))
  (set `self.Max Walk Speed` (`CharacterMovementComponent.MaxWalkSpeed` _charactermovement))
  (set `self.Max Acceleration` (`CharacterMovementComponent.MaxAcceleration` _charactermovement))
  (set `self.Rotation Rate` (`CharacterMovementComponent.RotationRate` _charactermovement))
  (bind _mesh (`Character.Mesh` _asbp_combat_character))
  (`self.Dash Setup` _mesh _charactermovement 100000000.0 (* _dash_distance _dash_rate) (struct :`Yaw` 100000000.0))
  (`KismetSystemLibrary.Delay` (* (/ 1.0 (`/Game/Variant_Combat/Blueprints/BP_CombatCharacter.Time Stop Dilation` _asbp_combat_character)) 0.1))
  (`AbilitySystemBlueprintLibrary.SendGameplayEventToActor` _asbp_combat_character (`self.Dash Tag`))
  (`AbilityTask_WaitGameplayEvent.WaitGameplayEvent` (struct :`TagName` "GameplayAbilities.EndDash") null
    (:`EventReceived`
      (`self.Dash Setup` _mesh _charactermovement (`self.Max Acceleration`) (`self.Max Walk Speed`) (`self.Rotation Rate`) true)
      (`self.K2_EndAbility`))))